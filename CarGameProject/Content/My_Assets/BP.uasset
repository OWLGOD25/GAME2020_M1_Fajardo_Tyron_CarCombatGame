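; Turret Blueprint meant to turn its top toward a player-tagged actor that enters its detection sphere.
; Sphere overlap stores the actor as Target, with no code to clear it.
; TrackTarget, which nothing here calls, starts a looping one-second timer for Targeting.
; Each Targeting call interpolates the top's relative yaw toward the look-at rotation by one frame's delta time, ignoring pitch and roll.
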(event OnComponentBeginOverlap(Sphere)
  (params (OverlappedComponent :type Primitive%20Component%20Object%20Reference) (OtherActor :type Actor%20Object%20Reference) (OtherComp :type Primitive%20Component%20Object%20Reference) (OtherBodyIndex :type Integer) (bFromSweep :type Boolean) (SweepResult :type Hit%20Result%20Structure%20%28by%20ref%29))
  ;[0.15 0.15 0.15 0.5] Trigger detection when player is close
  (Utilities|IsValid OtherActor
    (:Is%20Valid
      (if (Actor|ActorHasTag OtherActor "Player")
        (Variables|Default|SetTarget%20 OtherActor)))))

(event Custom|Track%20Target
  ;[0.15 0.15 0.15 0.5] Targeting system logic
  (bind _returnvalue (Utilities|Time|SetTimerbyEvent (delegate Custom|Targeting) 1.0 true true))
  (Variables|Default|SetTimerRef _returnvalue))

(event Custom|Targeting
  (bind _target_ (Variables|Default|GetTarget%20))
  ;[0.15 0.15 0.15 0.5] Targeting system logic
  (Utilities|IsValid _target_
    (:Is%20Valid
      (Transformation|SetRelativeRotation (Variables|Default|GetTurret%20top) (Math|Rotator|MakeRotator 0.0 0.0 (.yaw (Math|Interpolation|RInterpTo (Variables|/Script/Engine.SceneComponent|GetRelativeRotation (Variables|Default|GetTurret%20top)) (Math|Rotator|FindLookatRotation (Transformation|GetActorLocation) (Transformation|GetActorLocation _target_)) (Utilities|Time|GetWorldDeltaSeconds) 1.0))) false false))))

(event EventBeginPlay)

(event Collision|EventActorBeginOverlap
  (params (OtherActor :type Actor%20Object%20Reference)))

(event EventTick
  (params (DeltaSeconds :type Float%20%28single-precision%29)))

(fn ConstructionScript)