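; Turret actor that turns and fires TurretBullet actors when it senses the off-road car pawn.
; PawnSensing sightings set the actor's rotation from a look-at computed from the car toward the turret, then spawn a bullet after a short delay.
; Each sighting also sets a looping Fire timer, never cleared here, which keeps spawning bullets at the Tragectory component's transform.
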(event OnSeePawn(PawnSensing)
  (params (Pawn :type Pawn%20Object%20Reference))
  ;[0.15 0.15 0.15 0.5] Turret Targeting logic
  (Utilities|Casting|CastToBP_VehicleAdvOffroadCar Pawn)
  (Transformation|SetActorRotation (Math|Rotator|FindLookatRotation (Transformation|GetActorLocation Pawn) (Transformation|GetActorLocation)))
  (Utilities|Time|SetTimerbyFunctionName 0 "Fire" 1.0 true)
  (Utilities|FlowControl|Delay 0.2)
  (Game|SpawnActorfromClass "/Game/Importent_Assets/TurretBullet.TurretBullet_C" (Transformation|GetWorldTransform (Variables|Default|GetTragectory)) "AlwaysSpawn" "MultiplyWithRoot" 0 0))

(event Custom|Fire
  ;[0.15 0.15 0.15 0.5] Turret Targeting logic
  ;;[0.15 0.15 0.15 0.5] Fire Logic
  (Game|SpawnActorfromClass "/Game/Importent_Assets/TurretBullet.TurretBullet_C" (Transformation|GetWorldTransform (Variables|Default|GetTragectory)) "AlwaysSpawn" "MultiplyWithRoot" 0 0))

(event Collision|EventActorBeginOverlap
  (params (OtherActor :type Actor%20Object%20Reference)))

(event EventTick
  (params (DeltaSeconds :type Float%20%28single-precision%29)))

(fn ConstructionScript)